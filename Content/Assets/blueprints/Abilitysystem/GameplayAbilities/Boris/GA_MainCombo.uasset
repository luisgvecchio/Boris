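; Gameplay Ability for Boris's main combo attack, aimed at the point under the mouse.
; On valid target data it turns the avatar toward the hit location through CombatInterface, then plays AM_BorisCombo from a variable start section.
; A montage gameplay event triggers StartCombo1.
; Montage completion ends the ability and calls FinishCombo, with no handling for interruption or cancellation.
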(event Ability|EventActivateAbility
  (bind _returnvalue (Ability|GetAvatarActorfromActorInfo))
  (bind _datahandle (|TargetDataUnderMouse)
    (:ValidData
      (bind _output_get (Variables|Default|SetTargetLocation (.Location (Collision|BreakHitResult (Ability|TargetData|GetHitResultfromTargetData _datahandle)))))
      (Development|PrintString (Utilities|GetDisplayName _returnvalue) true true "(R=1.000000,G=0.961818,B=0.110000,A=1.000000)")
      (bind _ascombat_interface (Utilities|Casting|CastToCombatInterface _returnvalue))
      (Class|CombatInterface|UpdateFacingTarget _ascombat_interface _output_get)
      (|PlayMontageandWaitProxy "None" "/Game/Assets/Characters/Boris/Animations/AM_BorisCombo.AM_BorisCombo" 1.0 (Variables|Default|GetStart%20Section) true 1.0 0.0 false
        (:then
          (Ability|Tasks|WaitGameplayEvent "(TagName=\"Event.Montage.BorisMainCombo\")" 0
            (:EventReceived
              (Class|BorisMeleeAttack|StartCombo1))))
        (:OnCompleted
          (Ability|EndAbility)
          (Class|BorisMeleeAttack|FinishCombo))))))