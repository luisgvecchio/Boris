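; Gameplay ability that toggles the inventory screen for Boris.
; Each activation flips a stored IsActive flag, then ends immediately, so open state and widget persist between activations.
; Opening caches character and controller, creates WBP_Inventory if needed and switches to game-and-UI input; closing removes it and restores game-only input.
; On ability end, it passes the widget reference to the character's InventoryBaseComponent.
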(event Ability|EventActivateAbility
  (if (Variables|Default|GetIsActive)
    (Variables|Default|SetIsActive false)
    (Widget|RemovefromParent (Variables|Default|GetInventoryWidget))
    (Input|SetInputModeGameOnly (Variables|Default|GetBPBorisPlayerController) false)
    (else
      (Variables|Default|SetIsActive true)
      (CallFunction|SetBorisCharacterRef)
      (Utilities|IsValid (Variables|Default|GetInventoryWidget)
        (:Is%20Valid
          _)
        (:Is%20Not%20Valid
          (bind _returnvalue (UserInterface|CreateWidget "/Game/Assets/blueprints/Inventory/WBP_Inventory.WBP_Inventory_C"))
          (Variables|Default|SetInventoryWidget _returnvalue)))
      (UserInterface|Viewport|AddtoViewport (Variables|Default|GetInventoryWidget) 0)
      (Input|SetInputModeGameandUI (Variables|Default|GetBPBorisPlayerController) (Variables|Default|GetInventoryWidget) "DoNotLock" false false)))
  (Ability|EndAbility))

(event Ability|EventOnEndAbility
  (params (bWasCancelled :type Boolean))
  (CallFunction|UpdateInventoryComponentWidgetRef))

(fn SetBorisCharacterRef
  (bind _asbp_boris_character (Utilities|Casting|CastToBP_BorisCharacter (Ability|GetAvatarActorfromActorInfo)))
  (bind _output_get (Variables|Default|SetBPBorisCharacter _asbp_boris_character))
  (bind _asboris_player_controller (Utilities|Casting|CastToBorisPlayerController (Pawn|GetController _output_get)))
  (Variables|Default|SetBPBorisPlayerController _asboris_player_controller))

(fn UpdateInventoryComponentWidgetRef
  (Variables|/Script/Boris.InventoryBaseComponent|SetInventoryWidget (Actor|GetComponentbyClass (Variables|Default|GetBPBorisCharacter) "/Script/Boris.InventoryBaseComponent") (Variables|Default|GetInventoryWidget)))