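; Gameplay ability for the main combo of Boris's Lanza weapon.
; On activation it gets target data under the mouse and turns the avatar toward the hit location through CombatInterface.
; It then plays the combo montage from StartSection and waits for the combo montage gameplay event to call StartAttack.
; When the montage completes, it ends the ability and calls FinishAtttack.
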(event Ability|EventActivateAbility
  (bind _datahandle (|TargetDataUnderMouse)
    (:ValidData
      (bind _output_get (Variables|Default|SetTargetLocation (.Location (Collision|BreakHitResult (Ability|TargetData|GetHitResultfromTargetData _datahandle)))))
      (bind _ascombat_interface (Utilities|Casting|CastToCombatInterface (Ability|GetAvatarActorfromActorInfo)))
      (Class|CombatInterface|UpdateFacingTarget _ascombat_interface _output_get)
      (|PlayMontageandWaitProxy "None" "/Game/Assets/Characters/Boris/Animations/AM_BorisCombo.AM_BorisCombo" 1.0 (Variables|Default|GetStart%20Section) true 1.0 0.0 false
        (:then
          (Ability|Tasks|WaitGameplayEvent "(TagName=\"Event.Montage.BorisMainCombo\")" 0
            (:EventReceived
              (Class|BorisDamageGameplayAbility|StartAttack))))
        (:OnCompleted
          (Ability|EndAbility)
          (Class|BorisDamageGameplayAbility|FinishAtttack))))))