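; Base gameplay ability for Boris's main combo attacks, playing a montage section aimed at the point under the mouse.
; On activation it reads cursor target data, turns the avatar toward it via CombatInterface, then starts the montage.
; Gameplay events drive the attack: the start tag calls StartAttack, while the finish tag, interruption or cancellation ends the ability.
; An IsActive flag guards against ending twice, and OnEndAbility always calls FinishAtttack.
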(event Ability|EventActivateAbility
  (Variables|Default|SetIsActive true)
  (bind _datahandle (|TargetDataUnderMouse)
    (:ValidData
      (bind _output_get (Variables|Default|SetTargetLocation (.Location (Collision|BreakHitResult (Ability|TargetData|GetHitResultfromTargetData _datahandle)))))
      (bind _ascombat_interface (Utilities|Casting|CastToCombatInterface (Ability|GetAvatarActorfromActorInfo)))
      (Class|CombatInterface|UpdateFacingTarget _ascombat_interface _output_get)
      (|PlayMontageandWaitProxy "None" (Variables|Default|GetMontage%20to%20Play) 1.0 (Variables|Default|GetAM_SectionName) true 1.0 0.0 false
        (:then
          (Ability|Tasks|WaitGameplayEvent (Variables|Default|GetStartAttackTag) 0
            (:then
              (Ability|Tasks|WaitGameplayEvent (Variables|Default|GetFinishAttackTag) 0
                (:EventReceived
                  (CallFunction|EndAbilityifActive))))
            (:EventReceived
              (Class|BorisDamageGameplayAbility|StartAttack))))
        (:OnInterrupted
          (CallFunction|EndAbilityifActive :!label _label))
        (:OnCancelled
          (goto _label))))))

(event Ability|EventOnEndAbility
  (params (bWasCancelled :type Boolean))
  (Class|BorisDamageGameplayAbility|FinishAtttack)
  (Variables|Default|SetIsActive false))

(fn EndAbilityifActive
  (if (Variables|Default|GetIsActive)
    (Ability|EndAbility)))