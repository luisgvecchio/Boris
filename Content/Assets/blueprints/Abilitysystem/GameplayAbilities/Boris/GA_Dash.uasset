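; Gameplay ability that makes Boris dash toward the mouse cursor's hit point, or along his forward vector when the cursor hits nothing.
; It normalizes the horizontal direction, turns him toward the cursor point and uses LaunchCharacter with the dash force, overriding only XY velocity.
; His hit collider's collision is disabled for a brief immunity window, and a CanDash flag plus delays holds the ability active until the cooldown ends.
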(event Ability|EventActivateAbility
  (if (Variables|Default|GetCanDash)
    (CallFunction|AddDashForce)
    (CallFunction|TurnOffCollisiononHitCollider)
    (Variables|Default|SetCanDash false)
    (Utilities|FlowControl|Delay (Variables|Default|GetInmunitytime))
    (CallFunction|TurnonCollisiononHitCollider)
    (Utilities|FlowControl|Delay (- (Variables|Default|GetDashCooldown) (Variables|Default|GetInmunitytime)))
    (Variables|Default|SetCanDash true)
    (Ability|EndAbility)
    (else
      (Ability|EndAbility))))

(event Ability|EventOnEndAbility
  (params (bWasCancelled :type Boolean)))

(fn GetCursorHit
  (bind _asboris_player_controller (Utilities|Casting|CastToBorisPlayerController (Pawn|GetController (Variables|Default|GetBPBorisCharacter)))
    (:then
      (bind _returnvalue (Class|BorisPlayerController|GetCursorHit _asboris_player_controller))
      (Variables|Default|SetMouseImpactPoint (.ImpactPoint (Collision|BreakHitResult _returnvalue))))
    (:CastFailed
      _))
  (return (.bBlockingHit (Collision|BreakHitResult _returnvalue))))

(fn SetDashDirectiontoCharacterForwardVector
  (Variables|Default|SetDashDirection (Transformation|GetActorForwardVector (Variables|Default|GetBPBorisCharacter))))

(fn SetDashDirectiontoCursorHitLocation
  (bind _bpborischaracter (Variables|Default|GetBPBorisCharacter))
  (bind _mouseimpactpoint (Variables|Default|GetMouseImpactPoint))
  (bind _returnvalue (Transformation|GetActorLocation _bpborischaracter))
  (bind _returnvalue_2 (- _mouseimpactpoint _returnvalue))
  (Variables|Default|SetDashDirection (Math|Vector|Normalize (Math|Vector|MakeVector (.x _returnvalue_2) (.y _returnvalue_2) 0.0)))
  (return))

(fn SetBorisCharacterRef
  (bind _asbp_boris_character (Utilities|Casting|CastToBP_BorisCharacter (Ability|GetAvatarActorfromActorInfo)))
  (Variables|Default|SetBPBorisCharacter _asbp_boris_character))

(fn SetDashDirectiontoCursorHitandRotate
  (CallFunction|SetDashDirectiontoCursorHitLocation)
  (Transformation|SetActorRotation (Variables|Default|GetBPBorisCharacter) (Math|Rotator|FindLookatRotation (Transformation|GetActorLocation (Variables|Default|GetBPBorisCharacter)) (Variables|Default|GetMouseImpactPoint))))

(fn LaunchCharacter
  (params (B :type Integer))
  (Character|LaunchCharacter (Variables|Default|GetBPBorisCharacter) (* (Variables|Default|GetDashDirection) B) true false))

(fn AddDashForce
  (CallFunction|SetBorisCharacterRef)
  (bind _bblockinghit (CallFunction|GetCursorHit))
  (if _bblockinghit
    (CallFunction|SetDashDirectiontoCursorHitandRotate)
    (else
      (CallFunction|SetDashDirectiontoCharacterForwardVector)))
  (CallFunction|LaunchCharacter (Variables|Default|GetDashForce)))

(fn TurnOffCollisiononHitCollider
  (Collision|SetCollisionEnabled (Class|CombatInterface|GetHitCollider (Variables|Default|GetBPBorisCharacter)) "NoCollision"))

(fn TurnonCollisiononHitCollider
  (Collision|SetCollisionEnabled (Class|CombatInterface|GetHitCollider (Variables|Default|GetBPBorisCharacter)) "QueryOnly"))