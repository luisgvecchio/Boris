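; Enemy melee attack gameplay ability that turns the avatar toward its combat target and plays the Lanzero attack montage.
; Montage gameplay events drive the attack window: the start event calls StartAttack, and the finish event ends the ability.
; Montage interruption or cancellation also ends it, guarded by an IsActive flag.
; OnEndAbility always calls FinishAtttack, and debug prints mark attack start and ability end.
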(event Ability|EventActivateAbility
  (Variables|Default|SetIsActive true)
  (CallFunction|GetCombatTargetAnFaceIt)
  (|PlayMontageandWaitProxy "None" "/Game/Assets/Characters/Lanzero/Animations/AM_Lanzero_Attack.AM_Lanzero_Attack" 1.0 "None" true 1.0 0.0 false
    (:then
      (Ability|Tasks|WaitGameplayEvent "(TagName=\"Event.Montage.EnemyMeleeStartAttack\")" 0 true
        (:then
          (Ability|Tasks|WaitGameplayEvent "(TagName=\"Event.Montage.EnemyMeleeFinishAttack\")" 0 true
            (:EventReceived
              (CallFunction|EndAbilityifActive))))
        (:EventReceived
          (Class|BorisDamageGameplayAbility|StartAttack)
          (Development|PrintString "Start Attack"))))
    (:OnInterrupted
      (CallFunction|EndAbilityifActive :!label _label))
    (:OnCancelled
      (goto _label))))

(event Ability|EventOnEndAbility
  (params (bWasCancelled :type Boolean))
  (Class|BorisDamageGameplayAbility|FinishAtttack)
  (Variables|Default|SetIsActive false)
  (Development|PrintString "EndAbility" true true "(R=0.756271,G=1.000000,B=0.000000,A=1.000000)"))

(fn EndAbilityifActive
  (if (Variables|Default|GetIsActive)
    (Ability|EndAbility)))

(fn GetCombatTargetAnFaceIt
  (bind _returnvalue (Ability|GetAvatarActorfromActorInfo))
  (bind _returnvalue_2 (Class|EnemyInterface|GetCombatTarget(Message) _returnvalue))
  (bind _ascombat_interface (Utilities|Casting|CastToCombatInterface _returnvalue))
  (Class|CombatInterface|UpdateFacingTarget _ascombat_interface (Transformation|GetActorLocation _returnvalue_2)))