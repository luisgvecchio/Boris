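; Test actor prototyping an expanding explosion sphere and the point on its surface closest to the player.
; BeginPlay caches the BP_BorisCharacter, then Tick projects the normalized direction to it onto the scaled radius.
; Debug spheres draw that point and the collision sphere.
; The radius grows by a fixed step each frame, independent of delta time, with overlap updates disabled.
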(event EventBeginPlay
  ;[0.03101 1 0] BEGIN PLAY - Just Getting my Charachter and saving it in a Variable in the Sphere (explotion) blueprint.
  (bind _returnvalue (Actor|GetActorOfClass "/Game/Assets/blueprints/Boris/BP_BorisCharacter.BP_BorisCharacter_C"))
  (Variables|Default|SetCharacter _returnvalue))

(event EventTick
  (params (DeltaSeconds :type Float%20%28single-precision%29))
  ;[0 1 0.2255] TICK
  ;;[1 0.1531 0.9727] Debug Sphere for the calculated closest point on the surface to the player
  (Rendering|Debug|DrawDebugSphere (+ (* (Math|Vector|Normalize (- (Transformation|GetActorLocation (Variables|Default|GetCharacter)) (Transformation|GetActorLocation))) (Components|Sphere|GetScaledSphereRadius (Variables|Default|GetSphere))) (Transformation|GetActorLocation)) 1e+01 12 "(R=0.899065,G=0.000000,B=1.000000,A=1.000000)" 0.0)
  ;;[1 0.109 0.08507] Drawing Debug Sphere that represents the Collision from the Sphere
  (Rendering|Debug|DrawDebugSphere (Transformation|GetActorLocation) (Components|Sphere|GetScaledSphereRadius (Variables|Default|GetSphere)) 32 "(R=1.000000,G=0.083486,B=0.000000,A=1.000000)" 0.0 1.0)
  ;;[1 0.9438 0.8429] Making the Sphere Radius bigger each frame by 0.5 units
  (Components|Sphere|SetSphereRadius (Variables|Default|GetSphere) (+ (Variables|/Script/Engine.SphereComponent|GetSphereRadius (Variables|Default|GetSphere)) 0.5) false))

(fn ConstructionScript)