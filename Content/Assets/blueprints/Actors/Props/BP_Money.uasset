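; BP_Money is a money pickup whose mesh and amount come from its MoneyData.
; On BeginPlay it binds itself to the TS_Test template sequence and loops it.
; Sphere overlap adds money to a BorisCharacter's inventory component and updates the WBP_Inventory widget.
; Any overlapping actor, not just Boris, also triggers the instant gameplay effect application and destroys the pickup.
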(event OnComponentBeginOverlap(Sphere)
  (params (OverlappedComponent :type Primitive%20Component%20Object%20Reference) (OtherActor :type Actor%20Object%20Reference) (OtherComp :type Primitive%20Component%20Object%20Reference) (OtherBodyIndex :type Integer) (bFromSweep :type Boolean) (SweepResult :type Hit%20Result%20Structure%20%28by%20ref%29))
  (Variables|Default|SetCollided%20Actor OtherActor)
  (CallFunction|AddMoneytoPlayerInventory)
  (Class|BorisEffectActor|ApplyEffecttoTarget (Variables|Default|GetCollided%20Actor) (Variables|Default|GetInstantGameplayEffectClass))
  (Actor|DestroyActor))

(event EventBeginPlay
  (bind (_outactor _returnvalue) (Class|TemplateSequencePlayer|CreateTemplateSequencePlayer "/Game/Assets/blueprints/Actors/Items/Weapons/TS_Test.TS_Test"))
  (Class|TemplateSequenceActor|SetBinding _outactor self true)
  (Class|MovieSceneSequencePlayer|PlayLooping _returnvalue -1))

(fn ConstructionScript
  (Components|StaticMesh|SetStaticMesh (Variables|Default|GetMoneySM) (.mesh (Variables|/Script/Boris.MoneyAssetTypes|GetMoneyType (Variables|Default|GetMoneyData)))))

(fn AddMoneytoPlayerInventory
  (bind _asboris_character (Utilities|Casting|CastToBorisCharacter (Variables|Default|GetCollided%20Actor)))
  (bind _returnvalue (Class|BorisCharacter|GetInventoryComponent _asboris_character))
  (Class|InventoryBaseComponent|AddMoney _returnvalue (.amount (Variables|/Script/Boris.MoneyAssetTypes|GetMoneyType (Variables|Default|GetMoneyData))))
  (bind _aswbp_inventory (Utilities|Casting|CastToWBP_Inventory (Variables|/Script/Boris.InventoryBaseComponent|GetInventoryWidget _returnvalue)))
  (bind _returnvalue_2 (Class|InventoryBaseComponent|GetMoneyamount _returnvalue))
  (Variables|/Game/Assets/blueprints/Inventory/WBP_Inventory.WBP_Inventory_C|SetMoney _aswbp_inventory _returnvalue_2))